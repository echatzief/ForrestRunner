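; Game mode for a runner game that builds a chain of random floor tiles when play begins.
; BeginPlay repeatedly calls AddNewTile, which spawns Floor1, Floor2 or Floor3 at NewSpawnPoint, with Floor1 weighted double through the switch default.
; Each new tile's attach point becomes the next NewSpawnPoint with zero rotation and unit scale, so tiles line up end to end.
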(event `self.ReceiveBeginPlay`
  (for _ (range 13)
    (`self.Add New Tile`)))

(fn `Add New Tile`
  (bind _new_spawn_point (`self.New Spawn Point`))
  (switch `int` (`KismetMathLibrary.RandomIntegerInRange` 0 3)
    (:`Default`
      (bind _returnvalue (`|SpawnActorFromClass` "/Game/Forrest/Architecture/Floor1.Floor1_C" _new_spawn_point "Undefined" "OverrideRootScale" null null :!label _label))
      (bind _asfloor_1 (cast `/Game/Forrest/Architecture/Floor1` _returnvalue))
      (bind _returnvalue_2 (`/Game/Forrest/Architecture/Floor1.GetAttachTransform` _asfloor_1))
      (set `self.New Spawn Point` (`KismetMathLibrary.MakeTransform` _returnvalue_2)))
    (:`0`
      (goto _label))
    (:`1`
      (bind _returnvalue_3 (`|SpawnActorFromClass` "/Game/Forrest/Architecture/Floor2.Floor2_C" _new_spawn_point "Undefined" "OverrideRootScale" null null))
      (bind _asfloor_2 (cast `/Game/Forrest/Architecture/Floor2` _returnvalue_3))
      (bind _returnvalue_4 (`/Game/Forrest/Architecture/Floor2.Get Attach Transform 2` _asfloor_2))
      (set `self.New Spawn Point` (`KismetMathLibrary.MakeTransform` _returnvalue_4)))
    (:`2`
      (bind _returnvalue_5 (`|SpawnActorFromClass` "/Game/Forrest/Architecture/Floor3.Floor3_C" _new_spawn_point "Undefined" "OverrideRootScale" null null))
      (bind _asfloor_3 (cast `/Game/Forrest/Architecture/Floor3` _returnvalue_5))
      (bind _returnvalue_6 (`/Game/Forrest/Architecture/Floor3.GetAttachTransform` _asfloor_3))
      (set `self.New Spawn Point` (`KismetMathLibrary.MakeTransform` _returnvalue_6)))))

(fn `UserConstructionScript`)